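; BP_Projectile is a physics-driven weapon projectile that can ricochet off surfaces.
; Launch sets the Sphere's linear velocity directly.
; On each hit, it removes the Sphere and destroys the actor after a short delay if speed is below MinimumVelocity or the forward-to-normal angle is below RicocheteAngle.
; Otherwise it keeps flying, with the Sphere rotated to face its current velocity.
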(event `self.ReceiveTick`
  (params (DeltaSeconds :type "Float (single-precision)")))

(event `self.Sphere.OnComponentHit`
  (params (HitComponent :type "PrimitiveComponent Object Reference") (OtherActor :type "Actor Object Reference") (OtherComp :type "PrimitiveComponent Object Reference") (NormalImpulse :type "Vector Structure") (Hit :type "HitResult Structure (by ref)"))
  (bind _sphere (`self.Sphere`))
  (if (< (`KismetMathLibrary.VSize` (`SceneComponent.GetComponentVelocity` _sphere)) (`self.MinimumVelocity`))
    (`ActorComponent.K2_DestroyComponent` (`self.Sphere`))
    (`KismetSystemLibrary.Delay` 0.5)
    (`self.K2_DestroyActor`)
    (elif (< (`KismetMathLibrary.DegAcos` (`KismetMathLibrary.Dot_VectorVector` (`SceneComponent.GetForwardVector` _sphere) Hit_Normal)) (`self.RicocheteAngle`))
      (`ActorComponent.K2_DestroyComponent` (`self.Sphere`))
      (`KismetSystemLibrary.Delay` 0.5)
      (`self.K2_DestroyActor`)
      (else
        (`SceneComponent.K2_SetWorldRotation` _sphere (`KismetMathLibrary.Conv_VectorToRotator` (`SceneComponent.GetComponentVelocity` _sphere)) false false)))))

(fn `Launch`
  (params (InitialVelocity :type "Vector Structure"))
  (locals (NewLocalVar :type "ConstraintInstanceAccessor Structure"))
  (`PrimitiveComponent.SetPhysicsLinearVelocity` (`self.Sphere`) InitialVelocity false "None"))

(fn `UserConstructionScript`)