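; Elephant gun weapon Blueprint, a child gun that inherits its attack and base reload behavior from its parent class.
; It extends the reload start and end functions to set the IsReloading flag on the skeletal mesh's ABP_ElephantGunReload anim instance.
; The Attack override, construction script and event graph add no logic of their own.
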(fn `AnimateReload`
  (`parent.AnimateReload`)
  (bind _asabp_elephant_gun_reload (cast `/Game/Weapons/Assets/ElephantGun/Animations/ABP_ElephantGunReload` (`SkeletalMeshComponent.GetAnimInstance` (`self.SkeletalMesh`))))
  (set `/Game/Weapons/Assets/ElephantGun/Animations/ABP_ElephantGunReload.IsReloading` true _asabp_elephant_gun_reload))

(fn `Attack`
  (`parent.Attack`))

(fn `EndReloadAnimation`
  (`parent.EndReloadAnimation`)
  (bind _asabp_elephant_gun_reload (cast `/Game/Weapons/Assets/ElephantGun/Animations/ABP_ElephantGunReload` (`SkeletalMeshComponent.GetAnimInstance` (`self.SkeletalMesh`))))
  (set `/Game/Weapons/Assets/ElephantGun/Animations/ABP_ElephantGunReload.IsReloading` false _asabp_elephant_gun_reload))

(fn `UserConstructionScript`
  (`parent.UserConstructionScript`))